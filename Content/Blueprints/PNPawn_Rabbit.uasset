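; Rabbit pawn that switches between walk and sprint speeds and damages actors it runs into.
; BeginSprint and EndSprint set max walk speed and the IsSprint flag; while sprinting, Tick traces a short distance forward from the mesh and applies damage to the hit actor.
; Capsule hits apply the same damage regardless of sprint state.
; CanSeePlayerPawn line-traces forward by SightLength and reports any PNPlayerPawn hit.
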(event OnComponentHit(CapsuleComponent)
  (params (HitComponent :type Primitive%20Component%20Object%20Reference) (OtherActor :type Actor%20Object%20Reference) (OtherComp :type Primitive%20Component%20Object%20Reference) (NormalImpulse :type Vector :default "0, 0, 0") (Hit :type Hit%20Result%20Structure%20%28by%20ref%29))
  (Game|Damage|ApplyDamage OtherActor 1e+02 0 0))

(event EventBeginPlay
  (Variables|/Script/Engine.CharacterMovementComponent|SetMaxWalkSpeed (Variables|Character|GetCharacterMovement) (Variables|CharaSpec|GetWalkGroundSpeed)))

(event Collision|EventActorBeginOverlap
  (params (OtherActor :type Actor%20Object%20Reference)))

(event EventTick
  (params (DeltaSeconds :type Float%20%28single-precision%29))
  (bind _mesh (Variables|Character|GetMesh))
  (bind _returnvalue (Transformation|GetSocketLocation _mesh "None"))
  (if (Variables|Default|GetIsSprint)
    (bind _outhit (Collision|LineTraceByChannel _returnvalue (+ _returnvalue (* (Transformation|GetActorForwardVector) 5e+01)) "TraceTypeQuery3" false 0 "None"))
    (if true
      (Game|Damage|ApplyDamage (.HitActor (Collision|BreakHitResult _outhit)) 1e+02 0 0))))

(fn ConstructionScript)

(fn CanSeePlayerPawn
  (bind _returnvalue (Transformation|GetActorLocation))
  (bind _outhit (Collision|LineTraceByChannel _returnvalue (+ _returnvalue (* (Transformation|GetActorForwardVector) (Variables|CharaSpec|GetSightLength))) "TraceTypeQuery3" false 0 "ForOneFrame"))
  (return (.bSuccess (Utilities|Casting|CastToPNPlayerPawn (.HitActor (Collision|BreakHitResult _outhit)))) (.AsPNPlayer%20Pawn (Utilities|Casting|CastToPNPlayerPawn (.HitActor (Collision|BreakHitResult _outhit))))))

(fn BeginSprint
  (Variables|/Script/Engine.CharacterMovementComponent|SetMaxWalkSpeed (Variables|Character|GetCharacterMovement) (Variables|CharaSpec|GetSprintGroundSpeed))
  (Variables|Default|SetIsSprint true))

(fn EndSprint
  (Variables|/Script/Engine.CharacterMovementComponent|SetMaxWalkSpeed (Variables|Character|GetCharacterMovement) (Variables|CharaSpec|GetWalkGroundSpeed))
  (Variables|Default|SetIsSprint false))